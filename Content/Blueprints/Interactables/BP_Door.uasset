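; BP_Door is an interactable physics door whose two hinges can be broken by gadget hits.
; TriggerInteraction matches the hit component to a hinge cube and its physics constraint.
; An unbroken hinge spawns an explosion, swaps its material, breaks its constraint and is flagged in ConstraintsMap.
; Once every map entry is flagged, an impulse along the door's negative right vector knocks it loose.
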(event `/Game/Blueprints/Interfaces/IGadgetInteractable.TriggerInteraction`
  (params (GadgetType :type "/Game/Blueprints/Enums/EN_GadgetType Enum" :default "NewEnumerator0") (HitResult :type "HitResult Structure"))
  (`self.DetermineDoorHingeInteraction` GadgetType HitResult))

(fn `CheckForDoorHingeHit`
  (params (ComponentHit :type "PrimitiveComponent Object Reference"))
  (returns (DoorHinge :type "StaticMeshComponent Object Reference") (Constraint :type "PhysicsConstraintComponent Object Reference"))
  (if (== ComponentHit (`self.Cube2`))
    (return (`self.Cube2`) (`self.PhysicsConstraint`))
    (elif (== ComponentHit (`self.Cube1`))
      (return (`self.Cube1`) (`self.PhysicsConstraint1`))
      (else
        (return null null)))))

(fn `DetermineDoorHingeInteraction`
  (params (GadgetType :type "/Game/Blueprints/Enums/EN_GadgetType Enum" :default "NewEnumerator0") (HitResult :type "HitResult Structure"))
  (bind (_doorhinge _constraint) (`self.CheckForDoorHingeHit` (`.HitComponent` (`GameplayStatics.BreakHitResult` HitResult))))
  (bind (_value _returnvalue) (`BlueprintMapLibrary.Map_Find` (`self.ConstraintsMap`) _constraint))
  (bind (_returnvalue_location _returnvalue_rotation) (`KismetMathLibrary.BreakTransform` (`SceneComponent.K2_GetComponentToWorld` _doorhinge)))
  (switch `/Game/Blueprints/Enums/EN_GadgetType` GadgetType
    (:`NewEnumerator0`
      (if _returnvalue
        (if (and (not _value) (`KismetSystemLibrary.IsValid` _doorhinge))
          (`GameplayStatics.SpawnEmitterAtLocation` "/Game/SampleProject/StarterContent/Particles/P_Explosion.P_Explosion" _returnvalue_location _returnvalue_rotation)
          (`PrimitiveComponent.SetMaterial` _doorhinge 0 "/Game/SampleProject/StarterContent/VirtualReality/Materials/GenericHMDMaterial.GenericHMDMaterial")
          (`PhysicsConstraintComponent.BreakConstraint` _constraint)
          (`BlueprintMapLibrary.Map_Add` (`self.ConstraintsMap`) _constraint true)
          (bind _values (`BlueprintMapLibrary.Map_Values` (`self.ConstraintsMap`)))
          (for _array_element _values
            (if (not _array_element)
              (return)))
          (`PrimitiveComponent.AddImpulse` (`self.Cube`) (* (`SceneComponent.GetRightVector` (`self.Cube`)) -1000.0) "None" false))))))

(fn `UserConstructionScript`
  (set `self.ConstraintsMap` (`|MakeMap` (`self.PhysicsConstraint`) false (`self.PhysicsConstraint1`))))