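; BP_Laser is a laser gadget that repeatedly zaps whatever its Arrow component points at.
; Activating it starts a looping FireLaser timer alongside the parent gadget logic, and deactivating clears that timer.
; Each shot line-traces on Visibility, spawns a small pooled explosion at the hit and sends an interaction message to actors implementing IGadgetInteractable.
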(event `self.ReceiveBeginPlay`)

(fn `ActivateGadget`
  (`parent.ActivateGadget`)
  (`KismetSystemLibrary.K2_SetTimer` null "FireLaser" 0.1 true))

(fn `DeactivateGadget`
  (`parent.DeactivateGadget`)
  (`KismetSystemLibrary.K2_ClearTimer` null "FireLaser"))

(fn `FireLaser`
  (locals (hitResult :type "HitResult Structure"))
  (bind _arrow (`self.Arrow`))
  (bind (_bblockinghit _binitialoverlap _time _distance _location _impactpoint _normal _impactnormal _physmat _hitactor) (`GameplayStatics.BreakHitResult` (`local.hitResult`)))
  (bind _returnvalue (`SceneComponent.K2_GetComponentLocation` _arrow))
  (bind (_outhit _returnvalue_2) (`KismetSystemLibrary.LineTraceSingle` _returnvalue (+ _returnvalue (* (`SceneComponent.GetForwardVector` _arrow) 1000000.0)) "TraceTypeQuery1"))
  (set `local.hitResult` _outhit)
  (if _returnvalue_2
    (`self.SpawnLaserHitEffect` (`local.hitResult`))
    (if (`KismetSystemLibrary.DoesImplementInterface` _hitactor "/Game/Blueprints/Interfaces/IGadgetInteractable.IGadgetInteractable_C")
      (message `/Game/Blueprints/Interfaces/IGadgetInteractable.TriggerInteraction` _hitactor "NewEnumerator0" (`local.hitResult`)))))

(fn `SpawnLaserHitEffect`
  (params (hitResult :type "HitResult Structure"))
  (bind (_bblockinghit _binitialoverlap _time _distance _location _impactpoint _normal _impactnormal) (`GameplayStatics.BreakHitResult` hitResult))
  (`GameplayStatics.SpawnEmitterAtLocation` "/Game/SampleProject/StarterContent/Particles/P_Explosion.P_Explosion" _location (`KismetMathLibrary.Conv_VectorToRotator` _impactnormal) (0.1 0.1 0.1) true "AutoRelease"))

(fn `UserConstructionScript`)